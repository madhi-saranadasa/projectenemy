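; BP_Blob is a Blob enemy Blueprint that supplies the visual feedback for being hit and dying.
; StartHitEffect plays a world camera shake at the actor's location and spawns a hit spark Niagara system attached to the capsule.
; StartDeathEffect spawns the blob death Niagara system at the bottom of the capsule.
; The graph holds no other active logic, and both events are triggered from outside it.
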(event EventBeginPlay)

(event Collision|EventActorBeginOverlap
  (params (OtherActor :type Actor%20Object%20Reference)))

(event EventTick
  (params (DeltaSeconds :type Float%20%28single-precision%29)))

(event EventStartDeathEffect
  (bind _capsulecomponent (Variables|Default|GetCapsuleComponent))
  (bind _returnvalue (Transformation|GetWorldLocation _capsulecomponent))
  (bind (_x _y _z) (Math|Vector|BreakVector _returnvalue))
  (Niagara|SpawnSystematLocation "/Game/NIagara/Systems/FXSYS_BlobDeath.FXSYS_BlobDeath" (Math|Vector|MakeVector _x _y (- _z (Variables|/Script/Engine.CapsuleComponent|GetCapsuleHalfHeight _capsulecomponent)))))

(event EventStartHitEffect
  (Camera|PlayWorldCameraShake "/Game/Blueprints/Framework/CameraShake.CameraShake_C" (Transformation|GetActorLocation) 0.0 1e+03)
  (Niagara|SpawnSystemAttached "/Game/FX/Hit/HitSpark_System.HitSpark_System" (Variables|Default|GetCapsuleComponent) "None" "0, 0, 0" "0, 0, 0" "KeepRelativeOffset" false))

(fn ConstructionScript)