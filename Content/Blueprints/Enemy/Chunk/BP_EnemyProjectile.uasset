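; Enemy bubble projectile that waits for a set delay after a muzzle effect, then launches forward with collision enabled and an attached bubble effect.
; On sphere overlap it sends enemy-sourced damage to the other actor, spawns a hit effect, stops, disables collision and destroys itself shortly after.
; InitializeProjectile makes the sphere ignore the given owner actor while moving.
; The component hit event is empty, and the enemy-filtering damage branches are disconnected.
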(event OnComponentBeginOverlap(SphereComp)
  (params (OverlappedComponent :type Primitive%20Component%20Object%20Reference) (OtherActor :type Actor%20Object%20Reference) (OtherComp :type Primitive%20Component%20Object%20Reference) (OtherBodyIndex :type Integer) (bFromSweep :type Boolean) (SweepResult :type Hit%20Result%20Structure%20%28by%20ref%29))
  (Class|PawnInterface|TakeDamage(Message) OtherActor self (.Location (Collision|BreakHitResult SweepResult)) true)
  (Niagara|SpawnSystematLocation "/Game/NIagara/Systems/FXSYS_BubbleHit.FXSYS_BubbleHit" (Transformation|GetActorLocation) (Transformation|GetActorRotation))
  (Components|Movement|StopMovementImmediately (Variables|Default|GetMoveComp))
  (Collision|SetCollisionEnabled (Variables|Default|GetSphereComp) "NoCollision")
  (Utilities|FlowControl|Delay 0.1)
  (Actor|DestroyActor))

(event OnComponentHit(SphereComp)
  (params (HitComponent :type Primitive%20Component%20Object%20Reference) (OtherActor :type Actor%20Object%20Reference) (OtherComp :type Primitive%20Component%20Object%20Reference) (NormalImpulse :type Vector :default "0, 0, 0") (Hit :type Hit%20Result%20Structure%20%28by%20ref%29)))

(event EventBeginPlay
  (CallFunction|ToggleParticle false)
  (Niagara|SpawnSystematLocation "/Game/NIagara/Systems/FXSYS_BubbleMuzzle.FXSYS_BubbleMuzzle" (Transformation|GetActorLocation) (Transformation|GetActorRotation))
  (Utilities|FlowControl|Delay (Variables|Default|GetDelayPeriod))
  (CallFunction|ToggleParticle true)
  (bind _returnvalue (Niagara|SpawnSystemAttached "/Game/NIagara/Systems/FXSYS_Bubble.FXSYS_Bubble" (Variables|Default|GetSphereComp) "None" "0, 0, 0" "0, 0, 0" "KeepRelativeOffset" false)))

(fn ConstructionScript)

(fn ToggleParticle
  (params (Activation :type Boolean))
  (if Activation
    (Game|Components|ProjectileMovement|SetVelocityinLocalSpace (Variables|Default|GetMoveComp) (* (Class|KismetMathLibrary|VectorForward) (Variables|Default|GetProjectileSpeed)))
    (Collision|SetCollisionEnabled (Variables|Default|GetSphereComp) "QueryOnly")
    (else
      (Game|Components|ProjectileMovement|SetVelocityinLocalSpace (Variables|Default|GetMoveComp) (Math|Vector|VectorZero))
      (Collision|SetCollisionEnabled (Variables|Default|GetSphereComp) "NoCollision"))))

(fn InitializeProjectile
  (params (MotherActor :type Actor%20Object%20Reference))
  (Collision|IgnoreActorwhenMoving (Variables|Default|GetSphereComp) MotherActor true))