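; BP_SlimeProjectile is an enemy slime projectile that damages what it overlaps, ignoring other EnemyCharacters.
; On spawn it plays a bubble muzzle effect, switching collision and speed off, then on around it via ToggleCollisionAndSpeed.
; The sphere's overlap sends TakeDamageMessage with the impact point and enemy-projectile damage type.
; Blocking hits and valid overlaps both disable the projectile, spawn a bubble hit effect and destroy it.
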(event OnComponentHit(SphereComp)
  (params (HitComponent :type Primitive%20Component%20Object%20Reference) (OtherActor :type Actor%20Object%20Reference) (OtherComp :type Primitive%20Component%20Object%20Reference) (NormalImpulse :type Vector :default "0, 0, 0") (Hit :type Hit%20Result%20Structure%20%28by%20ref%29))
  (Class|EnemyProjectile|ToggleCollisionandSpeed false)
  (Niagara|SpawnSystematLocation "/Game/NIagara/Systems/FXSYS_BubbleHit.FXSYS_BubbleHit" (Transformation|GetActorLocation) (Transformation|GetActorRotation))
  (Actor|DestroyActor))

(event OnComponentBeginOverlap(SphereComp)
  (params (OverlappedComponent :type Primitive%20Component%20Object%20Reference) (OtherActor :type Actor%20Object%20Reference) (OtherComp :type Primitive%20Component%20Object%20Reference) (OtherBodyIndex :type Integer) (bFromSweep :type Boolean) (SweepResult :type Hit%20Result%20Structure%20%28by%20ref%29))
  (Utilities|Casting|CastToEnemyCharacter OtherActor
    (:CastFailed
      (Class|PawnInterface|TakeDamage(Message) OtherActor self (.ImpactPoint (Collision|BreakHitResult SweepResult)) "ENEMYPROJ")
      (Class|EnemyProjectile|ToggleCollisionandSpeed false)
      (Niagara|SpawnSystematLocation "/Game/NIagara/Systems/FXSYS_BubbleHit.FXSYS_BubbleHit" (Transformation|GetActorLocation) (Transformation|GetActorRotation))
      (Actor|DestroyActor))))

(event EventBeginPlay
  (Class|EnemyProjectile|ToggleCollisionandSpeed false)
  (Niagara|SpawnSystematLocation "/Game/NIagara/Systems/FXSYS_BubbleMuzzle.FXSYS_BubbleMuzzle" (Transformation|GetActorLocation) (Transformation|GetActorRotation))
  (Class|EnemyProjectile|ToggleCollisionandSpeed true))

(fn ConstructionScript)