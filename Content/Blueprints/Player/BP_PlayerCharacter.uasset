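; BP_PlayerCharacter is the player character Blueprint, exposing events that trigger the visual effects for primary and secondary attacks.
; A toggle event activates or deactivates the charge particles from a boolean input.
; Separate events activate the primary and secondary charge flashes and attack particles, resetting all but the toggle's deactivation on each call.
; It holds no attack logic, and its construction script is empty.
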(event EventBeginPlay)

(event Collision|EventActorBeginOverlap
  (params (OtherActor :type Actor%20Object%20Reference)))

(event EventPlayPrimaryFlash
  (Components|Activation|Activate (Variables|Default|GetPrimaryChargeFlash) true))

(event EventPlaySecondaryFlash
  (Components|Activation|Activate (Variables|Default|GetSecondaryChargeFlash) true))

(event EventTick
  (params (DeltaSeconds :type Float%20%28single-precision%29)))

(event EventToggleChargeParticle
  (params (InputBool :type Boolean))
  (bind _chargeparticles (Variables|Default|GetChargeParticles))
  (if InputBool
    (Components|Activation|Activate _chargeparticles true)
    (else
      (Components|Activation|Deactivate _chargeparticles))))

(event EventPlayParticleAttack
  (Components|Activation|Activate (Variables|Default|GetPrimaryAttackParticles) true))

(event EventPlaySecondaryAttack
  (Components|Activation|Activate (Variables|Default|GetSecondaryAttackParticles) true))

(fn ConstructionScript)